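; Board Blueprint for a dice-driven board game that moves the player along a track of slots.
; The Result function passes a step count to StartPlayerMovement, which ignores it while moving and caps the target at the last slot.
; MoveToNextSlot recursively steps one slot at a time via a timeline lerp in XY.
; On arrival, Bonus and Malus slots shift the target two slots forward or back, while Normal ends movement and messages the dice.
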(event Custom|MoveToNextSlot
  (bind _playerref (Variables|Default|GetPlayerRef))
  (bind _returnvalue (Transformation|GetActorLocation _playerref))
  (if (== (Variables|Default|GetCurrentSlotIndex) (Variables|Default|GetTargetSlotIndex))
    (switch Utilities|FlowControl|Switch|SwitchonE_SlotType (Variables|/Game/Blueprints/BP_Slot.BP_Slot_C|GetSlotTypeRef (Utilities|Array|Get(acopy) (Variables|Default|GetSlots) (Variables|Default|GetCurrentSlotIndex)))
      (:NewEnumerator0
        (Variables|Default|SetIsMoving false)
        (Class|BPI|ThrowDice(Message) (Variables|Default|GetDiceRef) true))
      (:NewEnumerator1
        (Variables|Default|SetTargetSlotIndex (Math|Integer|Min(Integer) (+ (Variables|Default|GetCurrentSlotIndex) 2) (- (Utilities|Array|Length (Variables|Default|GetSlots)) 1)))
        (CallFunction|MovetoNextSlot :!label _label))
      (:NewEnumerator2
        (Variables|Default|SetTargetSlotIndex (Math|Integer|Min(Integer) (- (Variables|Default|GetCurrentSlotIndex) 2) (- (Utilities|Array|Length (Variables|Default|GetSlots)) 1)))
        (goto _label)))
    (else
      (if (< (Variables|Default|GetCurrentSlotIndex) (Variables|Default|GetTargetSlotIndex))
        (Variables|Default|SetNextSlotIndex (+ (Variables|Default|GetCurrentSlotIndex) 1))
        (else
          (Variables|Default|SetNextSlotIndex (- (Variables|Default|GetCurrentSlotIndex) 1))))
      (Variables|Default|SetStartLocation _returnvalue)
      (Variables|Default|SetTargetLocation (Math|Vector|MakeVector (.X (Math|Vector|BreakVector (Transformation|GetActorLocation (Utilities|Array|Get(acopy) (Variables|Default|GetSlots) (Variables|Default|GetNextSlotIndex))))) (.Y (Math|Vector|BreakVector (Transformation|GetActorLocation (Utilities|Array|Get(acopy) (Variables|Default|GetSlots) (Variables|Default|GetNextSlotIndex))))) (.Z (Math|Vector|BreakVector _returnvalue))))
      (bind _alpha (Timeline|TL_MovePlayer PlayFromStart)
        (:Update
          (Transformation|SetActorLocation (Variables|Default|GetPlayerRef) (Math|Vector|Lerp(Vector) (Variables|Default|GetStartLocation) (Variables|Default|GetTargetLocation) _alpha) false false))
        (:Finished
          (Variables|Default|SetCurrentSlotIndex (Variables|Default|GetNextSlotIndex))
          (CallFunction|MovetoNextSlot))))))

(event Custom|StartPlayerMovement
  (params (Steps :type Integer))
  (if (not (Variables|Default|GetIsMoving))
    (Variables|Default|SetTargetSlotIndex (Math|Integer|Min(Integer) (+ Steps (Variables|Default|GetCurrentSlotIndex)) (- (Utilities|Array|Length (Variables|Default|GetSlots)) 1)))
    (Variables|Default|SetIsMoving true)
    (CallFunction|MovetoNextSlot)))

(fn ConstructionScript)

(fn Result
  (params (Result :type Integer))
  (CallFunction|StartPlayerMovement Result)
  (return))