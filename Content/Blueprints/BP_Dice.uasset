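; BP_Dice is the die that lets the player roll a number from 1 to 6 with the Space Bar for a board-based game.
; It enables input on BeginPlay, and a permitted roll locks further throws, prints the random result and sends it to the board through ResultMessage.
; The ThrowDice event sets the throw permission again, intended for when the player has finished moving.
; The Result function is an empty stub.
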(event EventBeginPlay
  (Input|EnableInput 0))

(event EventThrowDice
  (params (CanThrow :type Boolean))
  ;[0.15 0.15 0.15 0.5] Quand le joueur a fini de se déplacer, le joueur peut tirer le dé
  (Variables|Default|SetCanThrowDice CanThrow))

(event Input|KeyboardEvents|SpaceBar
  (params (Key :type Key%20Structure :default "None"))
  ;[0.15 0.15 0.15 0.5] Permet de lancer le dé, vérification si le joueur est en déplacement
  (:Pressed
    (if (Variables|Default|GetCanThrowDice)
      (Variables|Default|SetCanThrowDice false)
      ;[0.15 0.15 0.15 0.5] Random du chiffre du dé
      (bind _output_get (Variables|Default|SetDiceResult (Math|Random|RandomIntegerinRange 1 6)))
      (Development|PrintString (Utilities|String|ToString(Integer) _output_get))
      ;[0.15 0.15 0.15 0.5] Envoi au Board
      (Class|BPI|Result(Message) (Variables|Default|GetBoardReference) _output_get))))

(fn ConstructionScript)

(fn Result
  (params (Result :type Integer))
  (return))